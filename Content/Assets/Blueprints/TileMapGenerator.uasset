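; TileMapGenerator is an actor Blueprint that spawns a grid of child actor components at runtime, as the basis of a tile map.
; On BeginPlay, nested loops over Height and Width add one component per cell, spaced 100 units apart, with Height along X and Width along Y.
; A running Count is incremented and printed for each tile, and the construction script is empty.
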(event EventBeginPlay
  (for _index (range 0 (- (Variables|Default|Getheight) 1))
    (for _index_2 (range 0 (- (Variables|Default|Getwidth) 1))
      (AddComponent|AddChildActorComponent false (Math|Transform|MakeTransform (Math|Vector|MakeVector (Math|Conversions|ToFloat(Integer) (* _index 100)) (Math|Conversions|ToFloat(Integer) (* _index_2 100)) 0.0)))
      (bind _output_get (Variables|Default|Setcount (+ (Variables|Default|Getcount) 1)))
      (Development|PrintString (Utilities|String|ToString(Integer) _output_get)))))

(fn ConstructionScript)