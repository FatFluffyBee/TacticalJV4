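; Grid actor that spawns a square of BP_GridBloc tiles and takes two tile selections as path endpoints, with a cancel input that resets them.
; The second selection runs PathFinder, whose result gets the selected material.
; PathFinder is an unfinished step-cost search using open/closed lists, a hand-written sort and flat-index/XY conversion.
; It probes only diagonal neighbors, never checks the closed list and returns a single cell rather than a route.
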(event Custom|GridSelected
  (params (Case%201 :type BP%20Grid%20Bloc%20Object%20Reference))
  (Utilities|IsValid (Variables|Default|GetCase%201)
    (:Is%20Valid
      (bind _output_get (Variables|Default|SetCase%202 Case%201))
      (bind _path (CallFunction|PathFinder (stale _output_get_2) _output_get (Variables|Default|GetSquareSize) (Variables|Default|GetGridArray)))
      (for _array_element _path
        (bind _asbp_grid_bloc (Utilities|Casting|CastToBP_GridBloc _array_element))
        (Rendering|Material|SetMaterial (Variables|/Game/Assets/Blueprints/Grid/BP_GridBloc.BP_GridBloc_C|GetStaticMesh _asbp_grid_bloc) 0 "/Game/Assets/Art/Materials/M_GridSelected.M_GridSelected")))
    (:Is%20Not%20Valid
      (bind _output_get_2 (Variables|Default|SetCase%201 Case%201)))))

(event EventBeginPlay
  (Utilities|FlowControl|Sequence
    (:then_0
      (for _index (range 0 (Variables|Default|GetSquareSize))
        (for _index_2 (range 0 (Variables|Default|GetSquareSize))
          (bind _returnvalue (Game|SpawnActorfromClass "/Game/Assets/Blueprints/Grid/BP_GridBloc.BP_GridBloc_C" (Math|Transform|MakeTransform (Math|Vector|MakeVector (Math|Conversions|ToFloat(Integer) (* _index 100)) (Math|Conversions|ToFloat(Integer) (* _index_2 100)) 0.0) "0, 0, 0" "1.000000,1.000000,1.000000") "Undefined" 0 0))
          (Utilities|Array|Add (Variables|Default|GetGridArray) _returnvalue))))
    (:then_1
      (Input|EnableInput (Game|GetPlayerController 0)))))

(event Input|ActionEvents|InputActionInputAction_CancelAction
  (params (Key :type Key%20Structure))
  (:Pressed
    (Utilities|IsValid (Variables|Default|GetCase%201)
      (:Is%20Valid
        (bind _asbp_grid_bloc (Utilities|Casting|CastToBP_GridBloc (Variables|Default|GetCase%201)))
        (Default|Reset _asbp_grid_bloc)
        (Utilities|IsValid (Variables|Default|GetCase%202)
          (:Is%20Valid
            (bind _asbp_grid_bloc_2 (Utilities|Casting|CastToBP_GridBloc (Variables|Default|GetCase%202)))
            (Default|Reset _asbp_grid_bloc_2)
            (Variables|Default|SetCase%201 0)
            (Variables|Default|SetCase%202 0)))))))

(fn ConstructionScript)

(fn PathFinder
  (params (StartCase :type BP%20Grid%20Bloc%20Object%20Reference) (EndCase :type BP%20Grid%20Bloc%20Object%20Reference) (ArrayLength :type Integer) (Array :type Array%20of%20BP%20Grid%20Bloc%20Object%20References))
  (bind _neighbors (LocalVariables|GetNeighbors))
  (bind _open (LocalVariables|GetOpen))
  (Utilities|FlowControl|Sequence
    (:then_0
      (for (_array_element _array_index) (Variables|Default|GetGridArray)
        (if (== _array_element StartCase)
          (LocalVariables|SetStartIndex _array_index)
          (elif (== _array_element EndCase)
            (LocalVariables|SetEndIndex _array_index)
            (else
              (Development|PrintString "Hello"))))))
    (:then_1
      (bind (_x _y) (CallFunction|OutXandY (LocalVariables|GetStartIndex)))
      (Utilities|Array|Add (LocalVariables|GetOpen) (Utilities|Struct|MakeS_Pathfinder (Math|Vector2D|MakeVector2D (Math|Conversions|ToFloat(Integer) _x) (Math|Conversions|ToFloat(Integer) _y)) (Math|Vector2D|MakeVector2D (Math|Conversions|ToFloat(Integer) _x) (Math|Conversions|ToFloat(Integer) _y)) false 0)))
    (:then_2
      ;[1 1 1] Init
      (while (not (LocalVariables|GetFinished))
        (bind _sortedarray (CallFunction|SortArray (LocalVariables|GetOpen)))
        (LocalVariables|SetCurrent (Utilities|Array|Get(acopy) _sortedarray))
        (Utilities|Array|RemoveIndex _sortedarray)
        (Utilities|Array|Add (LocalVariables|GetClosed) (LocalVariables|GetCurrent))
        ;[1 1 1] Ajouter Neighbor to neigbors
        (bind _neighbor (CallFunction|SeekNeighbor "(X=1.000000,Y=1.000000)"))
        (Utilities|Array|Add (LocalVariables|GetNeighbors) _neighbor)
        (bind _neighbor_2 (CallFunction|SeekNeighbor "(X=-1.000000,Y=1.000000)"))
        (Utilities|Array|Add (LocalVariables|GetNeighbors) _neighbor_2)
        (bind _neighbor_3 (CallFunction|SeekNeighbor "(X=1.000000,Y=-1.000000)"))
        (Utilities|Array|Add (LocalVariables|GetNeighbors) _neighbor_3)
        (bind _neighbor_4 (CallFunction|SeekNeighbor "(X=-1.000000,Y=-1.000000)"))
        (Utilities|Array|Add (LocalVariables|GetNeighbors) _neighbor_4)
        ;[1 1 1] Check if neighbor is valid (in the range and not an obstacle
        (for (_array_element_2 _array_index_2) _neighbors
          (bind _flat (CallFunction|OutFlat (Math|Float|Truncate (.x (.position (Utilities|Array|Get(acopy) _neighbors _array_index_2)))) (Math|Float|Truncate (.y (.position (Utilities|Array|Get(acopy) _neighbors _array_index_2))))))
          (if (== _flat (LocalVariables|GetEndIndex))
            (LocalVariables|SetFinished true)
            (elif (Math|Boolean|ANDBoolean (> (.x (.Position (Utilities|Struct|BreakS_Pathfinder _array_element_2))) 0.0) (< (.x (.Position (Utilities|Struct|BreakS_Pathfinder _array_element_2))) (Variables|Default|GetSquareSize)) (> (.y (.Position (Utilities|Struct|BreakS_Pathfinder _array_element_2))) 0.0) (< (.y (.Position (Utilities|Struct|BreakS_Pathfinder _array_element_2))) (Variables|Default|GetSquareSize)))
              (bind _flat_2 (CallFunction|OutFlat (Math|Float|Truncate (.x (.Position (Utilities|Struct|BreakS_Pathfinder _array_element_2)))) (Math|Float|Truncate (.y (.Position (Utilities|Struct|BreakS_Pathfinder _array_element_2))))))
              (if (Utilities|IsValid (Utilities|Array|Get(acopy) (Variables|Default|GetGridArray) _flat_2))
                ;[1 1 1] Check if already registered, if yes check if modify, if not add it to open
                (if (== (Utilities|Array|FindItem (LocalVariables|GetOpen) (Utilities|Struct|MakeS_Pathfinder (.position (Utilities|Array|Get(acopy) (LocalVariables|GetNeighbors) _array_index_2)) "(X=0.000000,Y=0.000000)" false 0)) -1)
                  (Utilities|Array|Add (LocalVariables|GetOpen) (Utilities|Array|Get(acopy) (LocalVariables|GetNeighbors) _array_index_2))
                  (elif (>= (.cost (Utilities|Array|Get(acopy) _open (Utilities|Array|FindItem (LocalVariables|GetOpen) (Utilities|Struct|MakeS_Pathfinder (.position (Utilities|Array|Get(acopy) (LocalVariables|GetNeighbors) _array_index_2)) "(X=0.000000,Y=0.000000)" false 0)))) (.cost (Utilities|Array|Get(acopy) (LocalVariables|GetNeighbors) _array_index_2)))
                    (Utilities|Array|SetArrayElem _open _array_index_2 (Utilities|Struct|MakeS_Pathfinder (.position (Utilities|Array|Get(acopy) _open (Utilities|Array|FindItem (LocalVariables|GetOpen) (Utilities|Struct|MakeS_Pathfinder (.position (Utilities|Array|Get(acopy) (LocalVariables|GetNeighbors) _array_index_2)) "(X=0.000000,Y=0.000000)" false 0)))) (.parent (Utilities|Array|Get(acopy) (LocalVariables|GetNeighbors) _array_index_2)) false (.cost (Utilities|Array|Get(acopy) (LocalVariables|GetNeighbors) _array_index_2)))))))))))
      (bind _flat_3 (CallFunction|OutFlat (Math|Float|Truncate (.x (.position (LocalVariables|GetCurrent)))) (Math|Float|Truncate (.y (.position (LocalVariables|GetCurrent))))))
      (return (Utilities|Array|MakeArray (Utilities|Array|Get(acopy) (Variables|Default|GetGridArray) _flat_3))))))

(fn OutXandY
  (params (Flat :type Integer))
  (bind _squaresize (Variables|Default|GetSquareSize))
  (return (/ Flat _squaresize) (Math|Integer|%(Integer) Flat _squaresize)))

(fn SortArray
  (params (Array :type Array%20of%20S%20Pathfinder%20Structures))
  (for (_array_element _array_index) Array :!label _label
    (if (< _array_index (- (Utilities|Array|Length Array) 1))
      _
      (else
        ;[1 1 1] MEH
        (if (<= _array_index 1)
          _
          (else
            (return Array)))))
    (if (>= (.Cost (Utilities|Struct|BreakS_Pathfinder _array_element)) (.Cost (Utilities|Struct|BreakS_Pathfinder (Utilities|Array|Get(acopy) Array (+ _array_index 1)))))
      (bind _output_get (LocalVariables|SetTmp (Utilities|Array|Get(acopy) Array (+ _array_index 1))))
      (Utilities|Array|SetArrayElem Array (+ _array_index 1) (Utilities|Array|Get(acopy) Array (+ _array_index 1)))
      (Utilities|Array|SetArrayElem Array (.Cost (Utilities|Struct|BreakS_Pathfinder _array_element)) _output_get)
      (LocalVariables|SetVerif false)))
  (if (LocalVariables|GetVerif)
    (return 0)
    (else
      (LocalVariables|SetVerif true)
      (goto _label))))

(fn OutFlat
  (params (X :type Integer) (Y :type Integer))
  (return (+ (* (Variables|Default|GetSquareSize) X) Y)))

(fn SeekNeighbor
  (params (Offset :type Vector%202D%20Structure) (Current :type S%20Pathfinder%20Structure))
  (bind _returnvalue (+ (.position Current) ""))
  ;[1 1 1] Retourne une cell en fonction de current t d'un offset
  (bind _flat (CallFunction|OutFlat (Math|Float|Truncate (.x _returnvalue)) (Math|Float|Truncate (.y _returnvalue))))
  (return (Utilities|Struct|MakeS_Pathfinder (+ Offset (.position Current)) (.position Current) (Utilities|IsValid (Utilities|Array|Get(acopy) (Variables|Default|GetGridArray) _flat)) (+ (.cost Current) 1))))