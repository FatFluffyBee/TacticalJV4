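; BP_GridBloc is a single grid tile that reports mouse hover and click to the level's BP_Grid actor.
; On BeginPlay it traces downward, destroys itself if nothing is hit, and finds BP_Grid.
; Hover, selection and path flags drive a mesh material swap, with path taking priority over selected, then hover, then idle.
; Reset clears the flags and restores the idle material.
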(event OnClicked(StaticMesh)
  (params (TouchedComponent :type Primitive%20Component%20Object%20Reference) (ButtonPressed :type Key%20Structure :default "None"))
  (Variables|Default|SetIsSelected true)
  (bind _asbp_grid (Utilities|Casting|CastToBP_Grid (Variables|Default|GetBp_Grid)))
  (Default|GridSelected _asbp_grid self))

(event OnBeginCursorOver(StaticMesh)
  (params (TouchedComponent :type Primitive%20Component%20Object%20Reference))
  (Variables|Default|SetIsHovered true)
  (CallFunction|ChangeFeedback)
  (Default|GridHovered (Variables|Default|GetBp_Grid) self))

(event OnEndCursorOver(StaticMesh)
  (params (TouchedComponent :type Primitive%20Component%20Object%20Reference))
  (Variables|Default|SetIsHovered false)
  (CallFunction|ChangeFeedback))

(event Custom|Reset
  (Variables|Default|SetIsHovered false)
  (Variables|Default|SetIsPath false)
  (Variables|Default|SetIsSelected false)
  (Rendering|Material|SetMaterial (Variables|Default|GetStaticMesh) 0 "/Game/Assets/Art/Materials/M_GridIdle.M_GridIdle"))

(event Custom|ChangeFeedback
  (if (Variables|Default|GetIsPath)
    (Rendering|Material|SetMaterial (Variables|Default|GetStaticMesh) 0 "/Game/Assets/Art/Materials/M_GridPath.M_GridPath")
    (Development|PrintString "Changed")
    (elif (Variables|Default|GetIsSelected)
      (Rendering|Material|SetMaterial (Variables|Default|GetStaticMesh) 0 "/Game/Assets/Art/Materials/M_GridSelected.M_GridSelected")
      (elif (Variables|Default|GetIsHovered)
        (Rendering|Material|SetMaterial (Variables|Default|GetStaticMesh) 0 "/Game/Assets/Art/Materials/M_GridHover.M_GridHover")
        (else
          (Rendering|Material|SetMaterial (Variables|Default|GetStaticMesh) 0 "/Game/Assets/Art/Materials/M_GridIdle.M_GridIdle"))))))

(event EventOnClick)

(event EventBeginPlay
  (bind _returnvalue (Transformation|GetActorTransform))
  (Utilities|FlowControl|Sequence
    (:then_0
      (bind _returnvalue_2 (Collision|LineTraceByChannel (.location _returnvalue) (+ (.location _returnvalue) "0,0,-1000.000000") "TraceTypeQuery3" false 0 "None"))
      (if (not _returnvalue_2)
        (Actor|DestroyActor)))
    (:then_1
      (bind _returnvalue_3 (Actor|GetActorOfClass "/Game/Assets/Blueprints/Grid/BP_Grid.BP_Grid_C"))
      (Variables|Default|SetBp_Grid _returnvalue_3))))

(event EventOnHoverBegin)

(fn ConstructionScript)