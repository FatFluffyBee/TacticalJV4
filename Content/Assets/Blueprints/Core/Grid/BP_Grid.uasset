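; BP_Grid is a tile grid actor that builds a flat grid from a center location, tile size, tile count and shape.
; The construction script calls SpawnGrid, which clears old instances, then adds one instanced static mesh per tile in local space, stepping from the computed bottom-left corner.
; The shape enum names a DT_GridShapeData row supplying mesh, border material and mesh size for scaling, with an on-screen error if missing.
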(fn ConstructionScript
  (CallFunction|SpawnGrid (Variables|Default|GetGridCenterLocation) (Variables|Default|GetGridTileSize) (Variables|Default|GetGridTileCount) (Variables|Default|GetGridShape)))

(fn SpawnGrid
  (params (CenterLocation :type Vector) (TileSize :type Vector) (TileCount :type Vector%202D%20Structure) (Shape :type E_GridShape%20Enum :default "NewEnumerator0"))
  (bind _returnvalue (CallFunction|GetCurrentShapeData))
  (bind _instancedstaticmesh (Variables|Default|GetInstancedStaticMesh))
  (bind (_meshsize _mesh _meshmaterial _flatmesh _flatbordermaterial) (Utilities|Struct|BreakS_GridShapeData _returnvalue))
  (Variables|Default|SetGridCenterLocation CenterLocation)
  (Variables|Default|SetGridTileSize TileSize)
  (Variables|Default|SetGridTileCount TileCount)
  (Variables|Default|SetGridShape Shape)
  (CallFunction|DestroyGrid)
  (Components|StaticMesh|SetStaticMesh _instancedstaticmesh _flatmesh)
  (Rendering|Material|SetMaterial _instancedstaticmesh 0 _flatbordermaterial)
  (Variables|Default|SetGridBottomLeftCornerLocation (- (Variables|Default|GetGridCenterLocation) (* (/ (Variables|Default|GetGridTileCount) "(X=2.000000,Y=2.000000)") (Math|Conversions|ToVector2D(Vector) (Variables|Default|GetGridTileSize)))))
  (for _index (range 0 (- (Math|Float|Round (.x (Variables|Default|GetGridTileCount))) 1))
    (LocalVariables|SetX _index)
    (for _index_2 (range 0 (- (Math|Float|Round (.y (Variables|Default|GetGridTileCount))) 1))
      (LocalVariables|SetY _index_2)
      (LocalVariables|SetTileTransform (Math|Transform|MakeTransform (+ (Variables|Default|GetGridBottomLeftCornerLocation) (* (Variables|Default|GetGridTileSize) (Math|Vector|MakeVector (Math|Conversions|ToFloat(Integer) (LocalVariables|GetX)) (Math|Conversions|ToFloat(Integer) (LocalVariables|GetY)) 0.0))) "0, 0, 0" (/ (Variables|Default|GetGridTileSize) (.MeshSize (Utilities|Struct|BreakS_GridShapeData (CallFunction|GetCurrentShapeData))))))
      (Components|InstancedStaticMesh|AddInstance (Variables|Default|GetInstancedStaticMesh) (LocalVariables|GetTileTransform) false))))

(fn GetCurrentShapeData
  (bind _gridshape (Variables|Default|GetGridShape))
  (bind _returnvalue (Utilities|String|EnumtoString _gridshape))
  (bind _returnvalue_2 (Utilities|GetDataTableRow "/Game/Assets/Blueprints/Core/Grid/GridShapes/DT_GridShapeData.DT_GridShapeData" (Utilities|String|StringToName _returnvalue))
    (:then
      _)
    (:RowNotFound
      (Development|PrintString (Utilities|String|Append "Error : Row Not Found - " _returnvalue) true true "(R=1.000000,G=0.000000,B=0.276549,A=1.000000)" 5.0)))
  (return _returnvalue_2))

(fn DestroyGrid
  (Components|InstancedStaticMesh|ClearInstances (Variables|Default|GetInstancedStaticMesh)))