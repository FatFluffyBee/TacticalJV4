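; BP_PC is a player controller for a mouse-driven, turn-based game with two alternating players.
; On BeginPlay it shows the cursor and enables mouse click and hover events.
; Its EndTurn event increments the total turn count and toggles the active player number between one and two.
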(event Custom|EndTurn
  (Math|Integer|IncrementInt (Variables|Default|GetTotalTurn)
    (:%20%20
      (if (== (Variables|Default|GetNumberPlayer) 1)
        (Variables|Default|SetNumberPlayer 2)
        (else
          (Variables|Default|SetNumberPlayer 1))))))

(event EventBeginPlay
  (Variables|Default|SetbShowMouseCursor true)
  (Variables|Default|SetbEnableMouseOverEvents true)
  (Variables|Default|SetbEnableClickEvents true))

(fn ConstructionScript)